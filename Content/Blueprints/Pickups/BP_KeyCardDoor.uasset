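; Key card door interactable that opens only when the using player holds the matching key.
; Its UseAction override looks up DoorKey in CurrentKey on the player's BP_PlayerState.
; On success it runs the parent UseAction and destroys ObjectToOpen, so opening removes that actor rather than animating it.
; If the key check fails, it shows MissingKeyText on its TextRender.
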(fn `UseAction`
  (bind _objecttoopen (`self.ObjectToOpen`))
  (bind (_asbp_player_state _bsuccess) (cast `/Game/Blueprints/BP_PlayerState` (`Pawn.PlayerState` (`self.Player`)) :!pure true))
  (if _bsuccess
    (if (`BlueprintMapLibrary.Map_Find` (`/Game/Blueprints/BP_PlayerState.CurrentKey` _asbp_player_state) (`self.DoorKey`))
      (`parent.UseAction`)
      (`/Engine/EditorBlueprintResources/StandardMacros.IsValid` _objecttoopen
        (:`Is Valid`
          (`self.K2_DestroyActor` _objecttoopen)))
      (else
        (`TextRenderComponent.K2_SetText` (`self.TextRender`) (`self.MissingKeyText`))))))

(fn `UserConstructionScript`
  (`parent.UserConstructionScript`))