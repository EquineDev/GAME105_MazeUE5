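; BP_KeycardPickup is a usable pickup that grants the player a keycard.
; Its UseAction override casts the Player's PlayerState to BP_PlayerState and records the KeyCard as true in that state's CurrentKey collection.
; It then runs the parent use action and destroys itself; a failed cast stops everything, leaving the pickup in place.
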(fn `UseAction`
  (bind _asbp_player_state (cast `/Game/Blueprints/BP_PlayerState` (`Pawn.PlayerState` (`self.Player`))))
  (`BlueprintMapLibrary.Map_Add` (`/Game/Blueprints/BP_PlayerState.CurrentKey` _asbp_player_state) (`self.KeyCard`) true)
  (`parent.UseAction`)
  (`self.K2_DestroyActor`))

(fn `UserConstructionScript`
  (`parent.UserConstructionScript`))