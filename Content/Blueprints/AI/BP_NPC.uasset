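; NPC character that exposes movement, first-person look, weapon fire and interaction as events, with no decision logic or input bindings of its own.
; Movement follows the actor's forward and right vectors, look feeds controller pitch and yaw, and jump starts or stops on a pressed flag.
; Fire and Interact forward to WeaponObject and InteractObject when valid; SetupInteractions assigns the interact target.
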(event `self.MoveRight`
  (params (Value :type "Float (double-precision)"))
  ;[1 1 1] Movement
  (`self.AddMovementInput` (`self.GetActorRightVector`) Value))

(event `self.Jumping`
  (params (Pressed :type Boolean))
  ;[1 1 1] Movement
  (if Pressed
    (`self.Jump`)
    (else
      (`self.StopJumping`))))

(event `self.MoveFoward`
  (params (Value :type "Float (double-precision)"))
  ;[1 1 1] Movement
  (`self.AddMovementInput` (`self.GetActorForwardVector`) Value))

(event `self.LookPitch`
  (params (Value :type "Float (double-precision)"))
  ;[1 1 1] FPS look
  (`self.AddControllerPitchInput` Value))

(event `self.LookYaw`
  (params (Value :type "Float (double-precision)"))
  ;[1 1 1] FPS look
  (`self.AddControllerYawInput` Value))

(event `self.Fire`
  (bind _weaponobject (`self.WeaponObject`))
  ;[1 1 1] Fire Weapon
  (`/Engine/EditorBlueprintResources/StandardMacros.IsValid` _weaponobject
    (:`Is Valid`
      (`/Game/Blueprints/Components/BP_Weapon_Component_gun.FireWeapon` _weaponobject))))

(event `self.Interact`
  ;[1 1 1] Interactions
  (`/Engine/EditorBlueprintResources/StandardMacros.IsValid` (`self.InteractObject`)
    (:`Is Valid`
      (`/Game/Blueprints/Interfaces/BPI_InGameAction.Use` (`self.InteractObject`)))))

(fn `SetupInteractions`
  (params (Object :type "/Game/Blueprints/BP_ParentIntract Object Reference"))
  (set `self.InteractObject` Object))

(fn `UserConstructionScript`)