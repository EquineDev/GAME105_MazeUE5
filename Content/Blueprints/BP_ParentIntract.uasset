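; Parent Blueprint for interactable actors that display a text prompt when a tagged actor is nearby.
; The construction script applies UseText to a TextRender and toggles its visibility, which sphere overlap begin and end toggle again for actors matching Tag.
; Overlaps also call the empty OnEnter and OnExit hooks.
; The Use event calls UseAction, which by default only deactivates the text component.
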(event `self.Sphere.OnComponentBeginOverlap`
  (params (OverlappedComponent :type "PrimitiveComponent Object Reference") (OtherActor :type "Actor Object Reference") (OtherComp :type "PrimitiveComponent Object Reference") (OtherBodyIndex :type Integer) (bFromSweep :type Boolean) (SweepResult :type "HitResult Structure (by ref)"))
  ;[1 1 1] Toggle Tag
  (if (`self.ActorHasTag` OtherActor (`self.Tag`))
    (`SceneComponent.ToggleVisibility` (`self.TextRender`) false)
    (`self.On Enter`)))

(event `self.Sphere.OnComponentEndOverlap`
  (params (OverlappedComponent :type "PrimitiveComponent Object Reference") (OtherActor :type "Actor Object Reference") (OtherComp :type "PrimitiveComponent Object Reference") (OtherBodyIndex :type Integer))
  ;[1 1 1] Toggle Tag
  (if (`self.ActorHasTag` OtherActor (`self.Tag`))
    (`SceneComponent.ToggleVisibility` (`self.TextRender`) false)
    (`self.OnExit`)))

(event `/Game/Blueprints/BPI_InGameAction.Use`
  (`self.UseAction`))

(fn `On Enter`)

(fn `OnExit`)

(fn `UseAction`
  (`ActorComponent.SetActive` (`self.TextRender`) false false))

(fn `UserConstructionScript`
  (`TextRenderComponent.K2_SetText` (`self.TextRender`) (`self.UseText`))
  (`SceneComponent.ToggleVisibility` (`self.TextRender`) false))