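; BP_Player is the first-person player character, handling movement, jumping and mouse-look style camera input.
; Forward and right axis inputs add movement along the actor's own vectors, while pitch and yaw inputs feed the controller's rotation.
; The jump input starts a jump on press and stops it on release.
; Fire and Interact events exist but are empty, as are BeginPlay, Tick and the construction script.
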(event `/Game/Blueprints/BPI_PlayerInterface.MoveRight`
  (params (Value :type "Float (double-precision)"))
  ;[1 1 1] Movement
  (`self.AddMovementInput` (`self.GetActorRightVector`) Value))

(event `/Game/Blueprints/BPI_PlayerInterface.Jumping`
  (params (Pressed :type Boolean))
  ;[1 1 1] Movement
  (if Pressed
    (`self.Jump`)
    (else
      (`self.StopJumping`))))

(event `/Game/Blueprints/BPI_PlayerInterface.MoveFoward`
  (params (Value :type "Float (double-precision)"))
  ;[1 1 1] Movement
  (`self.AddMovementInput` (`self.GetActorForwardVector`) Value))

(event `/Game/Blueprints/BPI_PlayerInterface.LookPitch`
  (params (Value :type "Float (double-precision)"))
  ;[1 1 1] FPS look
  (`self.AddControllerPitchInput` Value))

(event `/Game/Blueprints/BPI_PlayerInterface.LookYaw`
  (params (Value :type "Float (double-precision)"))
  ;[1 1 1] FPS look
  (`self.AddControllerYawInput` Value))

(event `/Game/Blueprints/BPI_PlayerInterface.Fire`)

(event `/Game/Blueprints/BPI_PlayerInterface.Interact`)

(fn `UserConstructionScript`)