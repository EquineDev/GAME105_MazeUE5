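; Player state Blueprint that tracks the player's lives and score during a game.
; UpdateLives and UpdateScore add a delta, then refresh the in-game UI widget through a cast to BP_Playercontroller.
; When lives reach exactly zero, it prints "Game Over" and opens the GameOver level.
; ResetGameData restores default lives and score, refreshes both UI texts and clears CurrentKey if the controller cast succeeds.
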(event `/Game/Blueprints/Interfaces/BPI_StateUpdate.UpdateLives`
  (params (Value :type Integer))
  (bind (_asbp_playercontroller _bsuccess) (cast `/Game/Blueprints/BP_Playercontroller` (`self.GetPlayerController`) :!pure true))
  ;[1 1 1] UpdateLives
  (set `self.PlayerLives` (+ Value (`self.PlayerLives`)))
  (if (== (`self.PlayerLives`) 0)
    (`KismetSystemLibrary.PrintString` "Game Over")
    (`GameplayStatics.OpenLevelBySoftObjectPtr` "/Game/Maps/GameOver.GameOver")
    (elif _bsuccess
      (`/Game/UMG/WBP_InGameUI.Set Game Live Text` (`/Game/Blueprints/BP_Playercontroller.WBP_InGameUI` _asbp_playercontroller)))))

(event `/Game/Blueprints/Interfaces/BPI_StateUpdate.UpdateScore`
  (params (Value :type Integer))
  (bind (_asbp_playercontroller _bsuccess) (cast `/Game/Blueprints/BP_Playercontroller` (`self.GetPlayerController`) :!pure true))
  ;[1 1 1] UpdateScore
  (set `self.GameScore` (+ Value (`self.GameScore`)))
  (if _bsuccess
    (`/Game/UMG/WBP_InGameUI.Set Game Score Text` (`/Game/Blueprints/BP_Playercontroller.WBP_InGameUI` _asbp_playercontroller))))

(fn `ResetGameData`
  (bind (_asbp_playercontroller _bsuccess) (cast `/Game/Blueprints/BP_Playercontroller` (`self.GetPlayerController`) :!pure true))
  (bind _wbp_ingameui (`/Game/Blueprints/BP_Playercontroller.WBP_InGameUI` _asbp_playercontroller))
  (set `self.GameScore` (`self.DefaultScore`))
  (set `self.PlayerLives` (`self.DefaultLives`))
  (if _bsuccess
    (`/Game/UMG/WBP_InGameUI.Set Game Live Text` _wbp_ingameui)
    (`/Game/UMG/WBP_InGameUI.Set Game Score Text` _wbp_ingameui)
    (`BlueprintMapLibrary.Map_Clear` (`self.CurrentKey`))))

(fn `UserConstructionScript`)